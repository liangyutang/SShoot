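; BP_Bullet is a bullet actor that explodes on a timer rather than on impact.
; On BeginPlay it waits a short delay, then calls its Explore event, which spawns an explosion particle, applies full radial damage credited to the instigator, and destroys the actor.
; A debug sphere visualizes the damage radius, and the overlap event is an unused stub.
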(event Custom|Explore
  (bind _returnvalue (Transformation|GetActorLocation))
  (bind _damage_radius (Variables|Default|GetDamage%20Radius))
  (Effects|SpawnEmitteratLocation "/Game/WeaponEffects/Explosion/P_Explosion.P_Explosion" _returnvalue)
  (Game|Damage|ApplyRadialDamage (Variables|Default|GetBase%20Damage) _returnvalue _damage_radius 0 0 self (Game|GetInstigatorController) true "ECC_Visibility")
  (Rendering|Debug|DrawDebugSphere _returnvalue _damage_radius 12 "(R=0.207717,G=0.671462,B=1.000000,A=1.000000)" 1.0 1.0)
  (Actor|DestroyActor))

(event EventBeginPlay
  (Utilities|FlowControl|Delay 1.0)
  (CallFunction|Explore))

(event Collision|EventActorBeginOverlap
  (params (OtherActor :type Actor%20Object%20Reference)))

(fn ConstructionScript)